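; Game mode for a quiz game that builds the question pool and starts background music.
; On BeginPlay it reads save data from the game instance, plays music if enabled, then loads questions from the English or other-language DataTable by selected language.
; Questions are shuffled into a mixed array, and a language reset reruns this load.
; Helper functions advance the question index, find the next index with wraparound, and check for a win.
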(event Custom|PlayMusic
  (bind _asbp_game_instance (Utilities|Casting|CastToBP_GameInstance (Game|GetGameInstance)))
  (if (Variables|/Game/Quiz_Game/Blueprints/BP_GameInstance.BP_GameInstance_C|GetEnabledMusic _asbp_game_instance)
    (Utilities|IsValid (Variables|Default|GetMusic)
      (:Is%20Valid
        (Audio|Components|Audio|Stop (Variables|Default|GetMusic)))
      (:Is%20Not%20Valid
        _))
    (bind _returnvalue (Audio|SpawnSound2D "/Game/Quiz_Game/Audio/CUE_Crowd_Victory.CUE_Crowd_Victory" 1.0 1.0 0.0 0)) ; Set your background music here
    (Variables|Default|SetMusic _returnvalue)
    (else
      (Utilities|IsValid (Variables|Default|GetMusic)
        (:Is%20Valid
          (Audio|Components|Audio|Stop (Variables|Default|GetMusic)))))))

(event Custom|ResetLanguageFromSettings
  (Utilities|Array|Clear (Variables|Default|GetS_Questions))
  (switch Utilities|FlowControl|Switch|SwitchonE_Languages (Variables|/Game/Quiz_Game/Blueprints/BP_GameInstance.BP_GameInstance_C|GetSelected_Language (stale EventBeginPlay _asbp_game_instance))
    (:NewEnumerator0
      (CallFunction|AddQuestionsfromDataTable))
    (:NewEnumerator1
      (CallFunction|AddQuestionsfromDataTableOtherLang)))
  (CallFunction|RandomizeQuestions))

(event EventBeginPlay
  (bind _asbp_game_instance (Utilities|Casting|CastToBP_GameInstance (Game|GetGameInstance)))
  (Default|ReadSaveData _asbp_game_instance)
  (CallFunction|PlayMusic)
  (Utilities|Array|Clear (Variables|Default|GetS_Questions))
  (switch Utilities|FlowControl|Switch|SwitchonE_Languages (Variables|/Game/Quiz_Game/Blueprints/BP_GameInstance.BP_GameInstance_C|GetSelected_Language _asbp_game_instance)
    (:NewEnumerator0
      (CallFunction|AddQuestionsfromDataTable))
    (:NewEnumerator1
      (CallFunction|AddQuestionsfromDataTableOtherLang)))
  (CallFunction|RandomizeQuestions))

(fn ConstructionScript)

(fn RandomizeQuestions
  (bind _s_questions (Variables|Default|GetS_Questions))
  (Utilities|Array|Shuffle _s_questions)
  (Utilities|Array|Clear (Variables|Default|GetS_Questions_Mixed))
  (for _array_element _s_questions
    (Utilities|Array|Add (Variables|Default|GetS_Questions_Mixed) _array_element)))

(fn FindNextIndex
  (params (ItemToFind :type S%20Questions%20Structure%20%28by%20ref%29))
  (bind _s_questions_mixed (Variables|Default|GetS_Questions_Mixed))
  (bind _returnvalue (Utilities|Array|FindItem _s_questions_mixed ItemToFind))
  (bind _returnvalue_2 (Utilities|Array|LastIndex _s_questions_mixed))
  (if (== _returnvalue _returnvalue_2)
    (Variables|Default|SetIndexZero 0)
    (else
      (Variables|Default|SetIndexZero (Math|Integer|Clamp(Integer) (+ _returnvalue 1) 0 _returnvalue_2))))
  (return (Variables|Default|GetIndexZero)))

(fn IncreaseQuestionIndex
  (bind _output_get (Variables|Default|SetCurrentQuestion (+ (Variables|Default|GetCurrentQuestion) 1)))
  (return (Math|Integer|Clamp(Integer) _output_get 0 (Utilities|Array|LastIndex (Variables|Default|GetS_Questions)))))

(fn GameWon
  (params (LastQuestion :type Integer))
  (return (== LastQuestion (Variables|Default|GetTotalQuestions))))

(fn AddQuestionsfromDataTable
  (bind _outrownames (DataTable|GetDataTableRowNames "/Game/Quiz_Game/Blueprints/DT_Questions.DT_Questions"))
  (for _array_element _outrownames
    (bind _returnvalue (Utilities|GetDataTableRow "/Game/Quiz_Game/Blueprints/DT_Questions.DT_Questions" _array_element)
      (:then
        (Utilities|Array|Add (Variables|Default|GetS_Questions) (Utilities|Struct|MakeS_Questions (.Question (Utilities|Struct|BreakS_Questions _returnvalue)) (.Answers (Utilities|Struct|BreakS_Questions _returnvalue)) (.Correct (Utilities|Struct|BreakS_Questions _returnvalue)) (.ImageAnswer (Utilities|Struct|BreakS_Questions _returnvalue))))))))

(fn AddQuestionsfromDataTableOtherLang
  (bind _outrownames (DataTable|GetDataTableRowNames "/Game/Quiz_Game/Blueprints/DT_Questions_OtherLanguage.DT_Questions_OtherLanguage"))
  (for _array_element _outrownames
    (bind _returnvalue (Utilities|GetDataTableRow "/Game/Quiz_Game/Blueprints/DT_Questions_OtherLanguage.DT_Questions_OtherLanguage" _array_element)
      (:then
        (Utilities|Array|Add (Variables|Default|GetS_Questions) (Utilities|Struct|MakeS_Questions (.Question (Utilities|Struct|BreakS_Questions _returnvalue)) (.Answers (Utilities|Struct|BreakS_Questions _returnvalue)) (.Correct (Utilities|Struct|BreakS_Questions _returnvalue)) (.ImageAnswer (Utilities|Struct|BreakS_Questions _returnvalue))))))))